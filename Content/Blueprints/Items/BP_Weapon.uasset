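; BP_Weapon is a weapon item that the player picks up through interaction and swings to detect hits.
; Pickup calls EquipWeapon on BP_PlayerCharacter, then disables the mesh's collision and physics.
; Enabling attack collision starts a looping timer that box-traces between two trace points, using HitActors to register each actor once per attack window.
; Hits only print a debug message; no damage is applied and the DamageBox overlap event is empty.
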(event OnComponentBeginOverlap(DamageBox)
  (params (OverlappedComponent :type Primitive%20Component%20Object%20Reference) (OtherActor :type Actor%20Object%20Reference) (OtherComp :type Primitive%20Component%20Object%20Reference) (OtherBodyIndex :type Integer) (bFromSweep :type Boolean) (SweepResult :type Hit%20Result%20Structure%20%28by%20ref%29)))

(event Custom|EnableAttackCollision
  ;[0.15 0.15 0.15 0.5] Attack
  (Collision|SetCollisionEnabled (Variables|Default|GetDamageBox) "QueryOnly")
  (Variables|Default|SetIsTracing true)
  (Utilities|Array|Clear (Variables|Default|GetHitActors))
  (Utilities|Time|SetTimerbyFunctionName 0 "DoDamageTrace" 0.02 true))

(event Custom|DisableAttackCollision
  ;[0.15 0.15 0.15 0.5] Attack
  (Collision|SetCollisionEnabled (Variables|Default|GetDamageBox) "NoCollision")
  (Variables|Default|SetIsTracing false)
  (Utilities|Time|ClearTimerbyFunctionName 0 "DoDamageTrace")
  (Utilities|Array|Clear (Variables|Default|GetHitActors)))

(event EventBeginPlay
  (|CallParentFunction) ; This node is disabled and will not be called.\nDrag off pins to build functionality.
)

(event Collision|EventActorBeginOverlap
  (params (OtherActor :type Actor%20Object%20Reference))
  (|CallParentFunction OtherActor) ; This node is disabled and will not be called.\nDrag off pins to build functionality.
)

(event EventTick
  (params (DeltaSeconds :type Float%20%28single-precision%29))
  (|CallParentFunction DeltaSeconds) ; This node is disabled and will not be called.\nDrag off pins to build functionality.
)

(event EventPickUp
  (bind _itemmesh (Variables|Default|GetItemMesh))
  ;[0.15 0.15 0.15 0.5] Equip
  (bind _asbp_player_character (Utilities|Casting|CastToBP_PlayerCharacter (stale EventInteraction Interactor)))
  (Default|EquipWeapon _asbp_player_character self)
  (Development|PrintString (Utilities|String|Append (Variables|Default|GetItemName) " picked up"))
  (Variables|Default|SetIsPickedUp true)
  (Rendering|SetActorHiddenInGame false)
  (Collision|SetCollisionEnabled _itemmesh "NoCollision")
  (Physics|SetSimulatePhysics _itemmesh false))

(event EventInteraction
  (params (Interactor :type Actor%20Object%20Reference))
  ;[0.15 0.15 0.15 0.5] Equip
  (CallFunction|PickUp))

(fn ConstructionScript
  (|CallParentFunction))

(fn DoDamageTrace
  (bind _tracestart (Variables|Default|GetTraceStart))
  (bind _traceend (Variables|Default|GetTraceEnd))
  (bind _returnvalue (Transformation|GetWorldLocation _traceend))
  (bind _returnvalue_2 (Transformation|GetWorldLocation _tracestart))
  (bind _outhit (Collision|BoxTraceByChannel _returnvalue _returnvalue_2 (Math|Vector|MakeVector 1.0 1e+01 2.0) (Math|Rotator|FindLookatRotation _returnvalue _returnvalue_2) "TraceTypeQuery1" false 0 "ForDuration"))
  (if (.bBlockingHit (Collision|BreakHitResult _outhit))
    (Utilities|IsValid (.HitActor (Collision|BreakHitResult _outhit))
      (:Is%20Valid
        (if (not (Utilities|Array|ContainsItem (Variables|Default|GetHitActors) (.HitActor (Collision|BreakHitResult _outhit))))
          (Utilities|Array|Add (Variables|Default|GetHitActors) (.HitActor (Collision|BreakHitResult _outhit)))
          (Development|PrintString "Hit"))))))