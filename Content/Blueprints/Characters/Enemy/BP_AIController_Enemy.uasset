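; AI controller for enemy characters that runs their behavior tree and reacts to perceiving the player.
; Both BeginPlay and Possess cache the pawn and start BT_Enemy on BB_Enemy; Possess also hands the blackboard to the enemy.
; Perception updates set the player as TargetActor or, on loss, store its location and clear the target, switching enemy state either way.
; TryAttack starts an attack when the enemy reports it can.
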(event OnTargetPerceptionUpdated(AIPerception)
  (params (Actor :type Actor%20Object%20Reference) (Stimulus :type AI%20Stimulus%20Structure))
  (bind _enemy (Variables|Default|GetEnemy))
  (if (.bsuccessfullysensed Stimulus)
    (bind _asbp_player_character (Utilities|Casting|CastToBP_PlayerCharacter Actor))
    (AI|Components|Blackboard|SetValueasObject (Variables|Default|GetBlackboard) (Utilities|String|StringToName "TargetActor") _asbp_player_character)
    (Default|SetState _enemy "NewEnumerator1")
    (else
      (bind _asbp_player_character_2 (Utilities|Casting|CastToBP_PlayerCharacter Actor))
      (AI|Components|Blackboard|SetValueasVector (Variables|Default|GetBlackboard) (Utilities|String|StringToName "LastKnownPlayerPosition") (Transformation|GetActorLocation _asbp_player_character_2))
      (AI|Components|Blackboard|ClearValue (Variables|Default|GetBlackboard) (Utilities|String|StringToName "TargetActor"))
      (Default|SetState _enemy "NewEnumerator0"))))

(event EventBeginPlay
  (bind _asbp_enemy_character (Utilities|Casting|CastToBP_EnemyCharacter (Pawn|GetControlledPawn)))
  (Variables|Default|SetEnemy _asbp_enemy_character)
  (Class|AIController|UseBlackboard "/Game/Blueprints/Characters/Enemy/BB_Enemy.BB_Enemy")
  (AI|RunBehaviorTree "/Game/Blueprints/Characters/Enemy/BT_Enemy.BT_Enemy"))

(event EventTick
  (params (DeltaSeconds :type Float%20%28single-precision%29)))

(event EventPossess
  (params (PossessedPawn :type Pawn%20Object%20Reference))
  (bind _asbp_enemy_character (Utilities|Casting|CastToBP_EnemyCharacter PossessedPawn))
  (bind _output_get (Variables|Default|SetEnemy _asbp_enemy_character))
  (bind _blackboardcomponent (Class|AIController|UseBlackboard "/Game/Blueprints/Characters/Enemy/BB_Enemy.BB_Enemy"))
  (Variables|/Game/Blueprints/Characters/Enemy/BP_EnemyCharacter.BP_EnemyCharacter_C|SetBlackboard _output_get _blackboardcomponent)
  (AI|RunBehaviorTree "/Game/Blueprints/Characters/Enemy/BT_Enemy.BT_Enemy"))

(fn ConstructionScript)

(fn TryAttack
  (bind _enemy (Variables|Default|GetEnemy))
  (Utilities|IsValid _enemy
    (:Is%20Valid
      (bind _canattack (Default|CanAttack _enemy))
      (if _canattack
        (Default|StartAttack _enemy)))))