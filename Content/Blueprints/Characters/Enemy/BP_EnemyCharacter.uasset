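; Enemy character that spots the player, attacks with a socket-attached weapon spawned on BeginPlay, and reacts to damage.
; AI perception writes the target or last known position to the Blackboard and switches the pawn state, which SetState mirrors there.
; State gates attacks and hits; hits interrupt attack montages, apply damage through the attributes component and play reaction montage and sound.
; The component's OnDeath stops movement and destroys both enemy and weapon.
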(event OnDeath(BP_Attributes)
  ;[0.15 0.0177 0.02616 0.5] Combat System
  ;;[0.15 0.15 0.15 0.5] On Death
  (CallFunction|HandleDeath)
  (Development|PrintString "Enemy has been killed"))

(event OnTargetPerceptionUpdated(AIPerception)
  (params (Actor :type Actor%20Object%20Reference) (Stimulus :type AI%20Stimulus%20Structure))
  ;[0.15 0.5391 0.15 0.5] AI finding Player
  (Development|PrintString "Hello")
  (if (.bsuccessfullysensed Stimulus)
    (bind _asbp_player_character (Utilities|Casting|CastToBP_PlayerCharacter Actor))
    (AI|Components|Blackboard|SetValueasObject (Variables|Default|GetBlackboard) (Utilities|String|StringToName "TargetActor") _asbp_player_character)
    (CallFunction|SetState "NewEnumerator1")
    (else
      (AI|Components|Blackboard|SetValueasVector (Variables|Default|GetBlackboard) (Utilities|String|StringToName "LastKnownPlayerPosition") (Transformation|GetActorLocation _asbp_player_character))
      (AI|Components|Blackboard|ClearValue (Variables|Default|GetBlackboard) (Utilities|String|StringToName "TargetActor"))
      (CallFunction|SetState "NewEnumerator0"))))

(event Custom|SetState
  (params (New%20State :type E_PawnState%20Enum :default "NewEnumerator0"))
  ;[0.006852 0.07826 0.04048 0.5] Set Pawn State
  (bind _output_get (Variables|Default|SetPawnState New%20State))
  (AI|Components|Blackboard|SetValueasEnum (Variables|Default|GetBlackboard) (Utilities|String|StringToName "PawnState") _output_get))

(event Custom|HandleDeath
  (bind _charactermovement (Variables|Character|GetCharacterMovement))
  ;[0.15 0.0177 0.02616 0.5] Combat System
  ;;[0.15 0.15 0.15 0.5] Handle Death
  (CallFunction|SetState "NewEnumerator5")
  (Components|Movement|StopMovementImmediately _charactermovement)
  (Pawn|Components|CharacterMovement|DisableMovement _charactermovement)
  (Actor|DestroyActor)
  (Actor|DestroyActor (Variables|Default|GetEquippedWeapon)))

(event Custom|StartAttack
  ;[0.15 0.0177 0.02616 0.5] Combat System
  ;;[0.15 0.15 0.15 0.5] Attack
  (if (Utilities|Enum|Equal(Enum) (Variables|Default|GetPawnState) "NewEnumerator1")
    (CallFunction|SetState "NewEnumerator2")
    (Animation|PlayAnimMontage (Variables|Default|GetAM_Attack) 1.0 "None")
    (Development|PrintString "Enemy is attacking")))

(event EventBeginPlay
  ;[0.1321 0.07337 0.15 0.5] Spawn weapon in the hand
  (bind _returnvalue (Game|SpawnActorfromClass (Variables|Default|GetWeaponClass) (Transformation|GetSocketTransform (Variables|Character|GetMesh) "WeaponSocket" "RTS_World") "Undefined" "MultiplyWithRoot" 0 0))
  (CallFunction|EquipWeapon _returnvalue))

(event EventGetHit
  (params (HitLocation :type Vector :default "0, 0, 0") (Damage :type Float%20%28double-precision%29) (Instigator :type Actor%20Object%20Reference))
  ;[0.15 0.0177 0.02616 0.5] Combat System
  ;;[0.15 0.15 0.15 0.5] On Hit
  (if (Utilities|Enum|NotEqual(Enum) (Variables|Default|GetPawnState) "NewEnumerator5")
    (if (Utilities|Enum|NotEqual(Enum) (Variables|Default|GetPawnState) "NewEnumerator2")
      _
      (else
        (Animation|StopAnimMontage (Variables|Default|GetAM_Attack))))
    (Default|ApplyDamage (Variables|Default|GetBP_Attributes) Damage)
    (CallFunction|SetState "NewEnumerator3")
    (Animation|PlayAnimMontage (Variables|Default|GetAM_GetHit) 1.0 "None")
    (Audio|PlaySoundatLocation (Variables|Default|GetHitSound) (Transformation|GetActorLocation) "0, 0, 0" 1.0 1.0 0.0 0 0 0 0)
    (Development|PrintString "Enemy has been damaged")))

(fn ConstructionScript)

(fn CanAttack
  (bind _playerref (Variables|Default|GetPlayerRef))
  (Utilities|IsValid _playerref
    (:Is%20Valid
      (return (and (<= (Math|Vector|Distance(Vector) (Transformation|GetActorLocation) (Transformation|GetActorLocation _playerref)) (Variables|Default|GetAttackRange)) (Utilities|Enum|Equal(Enum) (Variables|Default|GetPawnState) "NewEnumerator1"))))))

(fn EquipWeapon
  (params (WeaponToEquip :type BP%20Weapon%20Object%20Reference))
  (bind _itemmesh (Variables|/Game/Blueprints/Items/BP_Item.BP_Item_C|GetItemMesh WeaponToEquip))
  (Utilities|IsValid WeaponToEquip
    (:Is%20Valid
      (Transformation|AttachComponentToComponent WeaponToEquip (Variables|Character|GetMesh) "WeaponSocket" "SnapToTarget" "SnapToTarget" "SnapToTarget" true)
      (bind _output_get (Variables|Default|SetEquippedWeapon WeaponToEquip))
      (Variables|/Game/Blueprints/Items/BP_Item.BP_Item_C|SetIsPickedUp _output_get true)
      (Rendering|SetActorHiddenInGame WeaponToEquip false)
      (Collision|SetCollisionEnabled _itemmesh "NoCollision")
      (Physics|SetSimulatePhysics _itemmesh false))))