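; BP_Attributes is an attributes Blueprint that holds a Health value and signals death when it runs out.
; GetHealth returns Health, while ApplyDamage subtracts the damage amount and calls OnDeath at zero or below.
; SetHealth stores only positive values; zero or negative input calls OnDeath and leaves Health unchanged.
; No clamping or repeat-death guard is present, and the event graph holds only disabled stubs.
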(event EventBeginPlay)

(event EventTick
  (params (DeltaSeconds :type Float%20%28single-precision%29)))

(fn GetHealth
  (return (Variables|Default|GetHealth)))

(fn SetHealth
  (params (NewValue :type Float%20%28double-precision%29))
  (if (<= NewValue 0.0)
    (Default|CallOnDeath)
    (else
      (Variables|Default|SetHealth NewValue))))

(fn ApplyDamage
  (params (DamageAmount :type Float%20%28double-precision%29))
  (bind _output_get (Variables|Default|SetHealth (- (Variables|Default|GetHealth) DamageAmount)))
  (if (<= _output_get 0.0)
    (Default|CallOnDeath)))