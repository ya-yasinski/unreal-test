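; Animation notify state for attacks that detects weapon hits on combat-capable actors.
; When the notify begins, it sphere-traces once between the mesh's WeaponBase and WeaponTip sockets across several object types, with debug drawing.
; If the hit actor implements BPI_Combat, it receives the GetHitMessage interface call.
; The tick override holds a disconnected copy of the same trace, so hits are not checked during the rest of the window.
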(fn ReceivedNotifyTick
  (params (MeshComp :type Skeletal%20Mesh%20Component%20Object%20Reference) (Animation :type Anim%20Sequence%20Base%20Object%20Reference) (FrameDeltaTime :type Float%20%28single-precision%29) (EventReference :type Anim%20Notify%20Event%20Reference%20Structure%20%28by%20ref%29)))

(fn ReceivedNotifyBegin
  (params (MeshComp :type Skeletal%20Mesh%20Component%20Object%20Reference) (Animation :type Anim%20Sequence%20Base%20Object%20Reference) (TotalDuration :type Float%20%28single-precision%29) (EventReference :type Anim%20Notify%20Event%20Reference%20Structure%20%28by%20ref%29))
  (bind _outhit (Collision|SphereTraceForObjects MeshComp (Transformation|GetSocketLocation MeshComp "WeaponBase") (Transformation|GetSocketLocation MeshComp "WeaponTip") 1e+01 (Utilities|Array|MakeArray "ObjectTypeQuery1" "ObjectTypeQuery2" "ObjectTypeQuery3" "ObjectTypeQuery4" "ObjectTypeQuery5" "ObjectTypeQuery6") false 0 "ForOneFrame" true "(R=1.000000,G=0.000000,B=0.000000,A=1.000000)" "(R=0.000000,G=1.000000,B=0.000000,A=1.000000)" 0.5))
  (if (Utilities|DoesObjectImplementInterface (.HitActor (Collision|BreakHitResult _outhit)) "/Game/Blueprints/Game/BPI_Combat.BPI_Combat_C")
    (Class|BPICombat|GetHit(Message) (.HitActor (Collision|BreakHitResult _outhit)))
    (return false)))