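; BP_Attributes is an attributes component that tracks health and signals death for whatever uses it.
; On BeginPlay it sets Health to MaxHealth, and ApplyDamage subtracts damage through SetHealth.
; SetHealth calls the OnDeath dispatcher when the new value is zero or below, leaving Health at its previous value, with no upper clamp or guard against repeated death calls.
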(event EventBeginPlay
  (CallFunction|SetHealth (Variables|Attributes|GetMaxHealth)))

(event EventTick
  (params (DeltaSeconds :type Float%20%28single-precision%29)))

(fn GetHealth
  (return (Variables|Attributes|GetHealth)))

(fn SetHealth
  (params (NewValue :type Float%20%28double-precision%29))
  (if (<= NewValue 0.0)
    (Default|CallOnDeath)
    (else
      (Variables|Attributes|SetHealth NewValue))))

(fn ApplyDamage
  (params (DamageAmount :type Float%20%28double-precision%29))
  (CallFunction|SetHealth (- (Variables|Attributes|GetHealth) DamageAmount)))